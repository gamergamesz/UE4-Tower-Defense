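; AI controller for enemies, apparently in a tower defense game, that gives them a goal location through a Blackboard.
; The construction script caches the TDGameState.
; On possess it sets up EnemyBB, writes the game state's Objective location to the objective key and runs the Enemy behavior tree.
; FindExit, not called here, can overwrite that key with the nearest MapExitPoint, or prints a warning when none exist.
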(event EventBeginPlay)

(event EventTick
  (params (DeltaSeconds :type Float%20%28single-precision%29)))

(event EventOnPossess
  (params (PossessedPawn :type Pawn%20Object%20Reference))
  (bind _blackboardcomponent (Class|AIController|UseBlackboard "/Game/Blueprints/Enemy/EnemyBB.EnemyBB"))
  (AI|Components|Blackboard|SetValueasVector _blackboardcomponent (Variables|Default|GetObjectiveKey) (Transformation|GetActorLocation (Variables|/Game/Blueprints/Gameplay/TDGameState.TDGameState_C|GetObjective (Variables|Default|GetGame%20State))))
  (AI|RunBehaviorTree "/Game/Blueprints/Enemy/Enemy.Enemy"))

(fn ConstructionScript
  (bind _astdgame_state (Utilities|Casting|CastToTDGameState (Game|GetGameState)))
  (Variables|Default|SetGame%20State _astdgame_state))

(fn FindExit
  (bind _outactors (Actor|GetAllActorsOfClass "/Game/Blueprints/Gameplay/Objectives/MapExitPoint.MapExitPoint_C"))
  (if (>= (Utilities|Array|LastIndex _outactors) 0)
    (for _array_element _outactors
      (if (< (Transformation|GetDistanceTo _array_element) (LocalVariables|GetClosest%20Exit%20Distance))
        (LocalVariables|SetClosest%20Exit _array_element)
        (LocalVariables|SetClosest%20Exit%20Distance (Transformation|GetDistanceTo _array_element))))
    (AI|Components|Blackboard|SetValueasVector (AI|GetBlackboard self) (Variables|Default|GetObjectiveKey) (Transformation|GetActorLocation (LocalVariables|GetClosest%20Exit)))
    (else
      (Development|PrintString "No exits in the map!"))))