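; Base tower defense enemy that steals food from a DefeatFood objective and escapes through a map exit.
; Touching food tells its AITest controller to find the exit and takes food up to its carry limit; touching a MapExitPoint destroys it.
; Lethal damage returns carried food to the GameState's objective, and any destruction removes it from the enemy count.
; Core logic sits in Basic functions that subclasses can reuse when overriding events.
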(event Collision|EventActorBeginOverlap
  (params (OtherActor :type Actor%20Object%20Reference))
  (if (== (Utilities|GetClass OtherActor) "/Game/Blueprints/Gameplay/Objectives/DefeatFood.DefeatFood_C")
    (bind _asaitest (Utilities|Casting|CastToAITest (Pawn|GetController)))
    (Default|FindExit _asaitest)
    (bind _asdefeat_food (Utilities|Casting|CastToDefeatFood OtherActor))
    (CallFunction|BasicTakeFood _asdefeat_food)
    (elif (== (Utilities|GetClass OtherActor) "/Game/Blueprints/Gameplay/Objectives/MapExitPoint.MapExitPoint_C")
      (Actor|DestroyActor))))

(event Game|Damage|EventAnyDamage
  (params (Damage :type Float%20%28single-precision%29) (DamageType :type Damage%20Type%20Object%20Reference) (InstigatedBy :type Controller%20Object%20Reference) (DamageCauser :type Actor%20Object%20Reference))
  (CallFunction|BasicDamage Damage DamageType InstigatedBy DamageCauser))

(event EventDestroyed
  ;[1 1 1] If you want to add more functionality to these sorts of events in another class, the event is completely overwritten by whatever the subclass has there, so add basic functions like these to the end of what you want to execute (since they're still accessible from enemy subclasses) or make new functions of your own based on what you need from the basics.
  (CallFunction|BasicDeath))

(event EventBeginPlay)

(fn ConstructionScript)

(fn BasicDeath
  ;[1 1 1] We could also make it give back the amount of food they took (if any) during this function
  (bind _astdgame_state (Utilities|Casting|CastToTDGameState (Game|GetGameState)))
  (Default|RemoveEnemy _astdgame_state))

(fn BasicDamage
  (params (Damage :type Float%20%28single-precision%29) (Damage%20Type :type Damage%20Type%20Object%20Reference) (Instigated%20By :type Controller%20Object%20Reference) (Damage%20Causer :type Actor%20Object%20Reference))
  (Development|PrintString "damage")
  (Variables|Default|SetHealth (- (Variables|Default|GetHealth) Damage))
  (if (<= (Variables|Default|GetHealth) 0.0)
    (bind _astdgame_state (Utilities|Casting|CastToTDGameState (Game|GetGameState)))
    (Default|GiveBackFood (Variables|/Game/Blueprints/Gameplay/TDGameState.TDGameState_C|GetObjective _astdgame_state) (Variables|Default|GetCurrentFoodAmount))
    (Actor|DestroyActor)))

(fn BasicTakeFood
  (params (Food :type Defeat%20Food%20Object%20Reference))
  (bind _amount_taken (Default|RemoveFood Food (Math|Integer|Min(Integer) (Variables|Default|GetFoodStealAmount) (- (Variables|Default|GetMaximumFoodAmount) (Variables|Default|GetCurrentFoodAmount)))))
  (Variables|Default|SetCurrentFoodAmount (+ _amount_taken (Variables|Default|GetCurrentFoodAmount)))
  (return _amount_taken))