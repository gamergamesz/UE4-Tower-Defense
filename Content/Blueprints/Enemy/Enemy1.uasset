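; Enemy1 is a basic enemy with character movement that walks toward a fixed point and can be killed by damage.
; On BeginPlay, its AI controller gets a Simple Move to Location order with a hardcoded goal.
; AnyDamage prints a debug message, subtracts from Health and destroys the actor at zero or below.
; Unconnected AI MoveTo and MoveUpdatedComponent nodes remain in the graph and never run.
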(event Game|Damage|EventAnyDamage
  (params (Damage :type Float%20%28single-precision%29) (DamageType :type Damage%20Type%20Object%20Reference) (InstigatedBy :type Controller%20Object%20Reference) (DamageCauser :type Actor%20Object%20Reference))
  ;[1 1 1] Modify to work with Damageable interface later? Or add it to function library?
  (Development|PrintString "damage")
  (Variables|Default|SetHealth (- (Variables|Default|GetHealth) Damage))
  (if (<= (Variables|Default|GetHealth) 0.0)
    (Actor|DestroyActor)))

(event EventBeginPlay
  (AI|Navigation|SimpleMovetoLocation (stale _returnvalue) (Math|Vector|MakeVector 15.0 0.0 0.0)))

(event EventActorBeginOverlap
  (params (OtherActor :type Actor%20Object%20Reference)))

(event EventTick
  (params (DeltaSeconds :type Float%20%28single-precision%29)))

(fn ConstructionScript)