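; Player controller for a tower defense game that adds the in-game menu on BeginPlay and handles mouse and keyboard input, much of it test code.
; Clicks and keys spawn towers or enemies at the deprojected mouse position flattened to zero height, or start a wave through TDGameState.
; Right-click toggles the PMSelection widget.
; Other inputs exercise event dispatcher binding with debug prints; a comment flags tower placement displaced by range-radius collision.
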(event Custom|CustomEvent_1
  ;[1 1 1] learning code
  (Development|PrintString "zxcvzxcvzxcv"))

(event Custom|CustomEvent_0
  ;[1 1 1] learning code
  (Development|PrintString "asdfasdffaasdf"))

(event EventBeginPlay
  (Input|EnableInput 0)
  (bind _returnvalue (UserInterface|CreateWidget "/Game/Blueprints/UI/Ingame_Menu.Ingame_Menu_C"))
  (UserInterface|Viewport|AddtoViewport _returnvalue 0))

(event EventTick
  (params (DeltaSeconds :type Float%20%28single-precision%29)))

(event Input|ActionEvents|InputActionshoot
  (params (Key :type Key%20Structure :default "AnyKey"))
  ;[1 1 1] learning code
  (:Pressed
    (Default|CallSomehing)))

(event Input|MouseEvents|RightMouseButton
  (params (Key :type Key%20Structure :default "AnyKey"))
  ;[1 1 1] on click testing
  (:Pressed
    (Utilities|FlowControl|FlipFlop
      (:A
        (bind _returnvalue (UserInterface|CreateWidget "/Game/Blueprints/UI/PMSelection.PMSelection_C"))
        (UserInterface|Viewport|AddtoViewport _returnvalue 0)
        (Development|PrintString "widget's on"))
      (:B
        (Widget|RemovefromParent _returnvalue)
        (Development|PrintString "widget's gone again")))))

(event Input|KeyboardEvents|Z
  (params (Key :type Key%20Structure :default "AnyKey"))
  (:Pressed
    (bind _astdgame_state (Utilities|Casting|CastToTDGameState (Game|GetGameState)))
    (Default|StartWave _astdgame_state)))

(event Input|MouseEvents|LeftMouseButton
  (params (Key :type Key%20Structure :default "AnyKey"))
  (bind _worldlocation (Game|Player|ConvertMouseLocationToWorldSpace))
  (bind (_x _y) (Math|Vector|BreakVector _worldlocation))
  (:Pressed
    ;[1 1 1] BUG: Something about colliding with the towers' range radius makes it so that if you try to spawn a tower near another one, it'll move to be outside of the towers' range if you have the collision handling set to be adjust to collisions
    (Game|SpawnActorfromClass "/Game/Blueprints/Towers/Tower1.Tower1_C" (Math|Transform|MakeTransform (Math|Vector|MakeVector _x _y 0.0)) "Undefined" 0 0)))

(event Input|KeyboardEvents|SpaceBar
  (params (Key :type Key%20Structure :default "AnyKey"))
  (bind _worldlocation (Game|Player|ConvertMouseLocationToWorldSpace))
  (bind (_x _y) (Math|Vector|BreakVector _worldlocation))
  (:Pressed
    (Game|SpawnActorfromClass "/Game/Blueprints/Enemy/BaseEnemy.BaseEnemy_C" (Math|Transform|MakeTransform (Math|Vector|MakeVector _x _y 0.0)) "Undefined" 0 0)))

(event Input|KeyboardEvents|Right
  (params (Key :type Key%20Structure :default "AnyKey"))
  ;[1 1 1] learning code
  (:Pressed
    (EventDispatchers|UnbindallEventsfromSomehing)
    (EventDispatchers|BindEventtoSomehing (delegate Custom|CustomEvent_1))))

(event Input|KeyboardEvents|Up
  (params (Key :type Key%20Structure :default "AnyKey"))
  ;[1 1 1] learning code
  (:Pressed
    (EventDispatchers|BindEventtoSomehing (delegate Custom|CustomEvent_0))))

(fn ConstructionScript)