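; Tower defense game state that runs enemy waves and tracks map resource locations and the player's resource total.
; StartWave and SpawnEnemyFromWave consume the EnemiesToSpawn queue through chained function-name timers, mapping type to class and retrying failed spawns immediately by recursion.
; RemoveEnemy calls EndWave at zero enemies, which schedules the next wave or prints victory.
; BeginPlay, Tick and DefeatCheck are empty, with the lose check left unwired.
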(event EventBeginPlay)

(event EventTick
  (params (DeltaSeconds :type Float%20%28single-precision%29)))

(fn ConstructionScript)

(fn EnemyClassSelector
  (params (Enemy%20Name :type String))
  (switch string Enemy%20Name
    (:Default
      (Development|PrintString "Base Enemy")
      (return "/Game/Blueprints/Enemy/BaseEnemy.BaseEnemy_C"))
    (:Crazy%20Ant
      (Development|PrintString "Crazy Ant")
      (return "/Game/Blueprints/Enemy/CrazyAnt.CrazyAnt_C"))))

(fn RemoveEnemy
  (bind _result (Math|Integer|DecrementInt (Variables|Default|GetEnemy%20Amount))
    (:%20%20
      (Development|PrintString (Utilities|String|ToString(Integer) (Variables|Default|GetEnemy%20Amount)))
      (if (<= _result 0)
        (CallFunction|EndWave)))))

(fn SpawnEnemyfromWave
  (bind _returnvalue (Utilities|Time|GetGameTimeinSeconds))
  (bind _wave_start_time (Variables|Default|GetWave%20Start%20Time))
  (bind _enemies_to_spawn (Variables|Default|GetEnemies%20to%20Spawn))
  (bind _minimum_spawn_time (Variables|Default|GetMinimum%20Spawn%20Time))
  (bind _enemies_to_spawn_2 (Variables|Default|GetEnemies%20to%20Spawn))
  (bind _item (Utilities|Array|Get(acopy) _enemies_to_spawn))
  (bind _item_2 (Utilities|Array|Get(acopy) _enemies_to_spawn_2))
  (bind (_wave _enemytype _location) (Utilities|Struct|BreakSpawningData _item_2))
  (bind _time (Utilities|Struct|BreakSpawningData _item))
  (bind _returnvalue_2 (+ _wave_start_time _time))
  (bind _returnvalue_3 (- _returnvalue_2 _returnvalue))
  (bind _returnvalue_4 (Math|Float|Max(Float) _returnvalue_3 _minimum_spawn_time))
  (bind _enemy_class (CallFunction|EnemyClassSelector _enemytype))
  (bind _returnvalue_5 (Game|SpawnActorfromClass _enemy_class (Transformation|GetActorTransform (Utilities|Array|Get(acopy) (Variables|Default|GetEnemy%20Spawn%20Locations) (- _location 1))) "Undefined" 0 0))
  (if (Utilities|IsValid _returnvalue_5)
    (Math|Integer|IncrementInt (Variables|Default|GetEnemy%20Amount)
      (:%20%20
        (Utilities|Array|RemoveIndex (Variables|Default|GetEnemies%20to%20Spawn))
        (bind _is_spawn_valid (CallFunction|CheckNextSpawn))
        (if _is_spawn_valid
          (Utilities|Time|SetTimerbyFunctionName 0 "Spawn Enemy from Wave" _returnvalue_4)
          (Development|PrintString (Utilities|String|Append "Next spawn in " (Utilities|String|ToString(Float) _returnvalue_4) " seconds."))
          (else
            (Development|PrintString "No enemies left for this wave.")))))
    (else
      (Development|PrintString "Failed to Spawn")
      ;[1 1 1] Try again
      (CallFunction|SpawnEnemyfromWave))))

(fn CheckNextSpawn
  (if (!= (Utilities|Array|LastIndex (Variables|Default|GetEnemies%20to%20Spawn)) -1)
    (return (>= (Variables|Default|GetCurrent%20Wave) (.Wave (Utilities|Struct|BreakSpawningData (Utilities|Array|Get(acopy) (Variables|Default|GetEnemies%20to%20Spawn))))))
    (else
      (return false))))

(fn EndWave
  ;[1 1 1] Execute victory things if true (call an event dispatcher? That way you can bind events in other classes to this)
  (if (and (== (Variables|Default|GetCurrent%20Wave) (Variables|Default|GetWave%20Amount)) (== (Utilities|Array|LastIndex (Variables|Default|GetEnemies%20to%20Spawn)) -1))
    (Development|PrintString "You won!")
    (elif (> (.Wave (Utilities|Struct|BreakSpawningData (Utilities|Array|Get(acopy) (Variables|Default|GetEnemies%20to%20Spawn)))) (Variables|Default|GetCurrent%20Wave))
      (Utilities|Time|SetTimerbyFunctionName 0 "Start Wave" (Variables|Default|GetNext%20Wave%20Delay)))))

(fn StartWave
  (bind _enemies_to_spawn (Variables|Default|GetEnemies%20to%20Spawn))
  (bind _item (Utilities|Array|Get(acopy) _enemies_to_spawn))
  (bind _time (Utilities|Struct|BreakSpawningData _item))
  (if (< (Variables|Default|GetCurrent%20Wave) (Variables|Default|GetWave%20Amount))
    (Math|Integer|IncrementInt (Variables|Default|GetCurrent%20Wave)
      (:%20%20
        (Variables|Default|SetWave%20Start%20Time (Utilities|Time|GetGameTimeinSeconds))
        (bind _is_spawn_valid (CallFunction|CheckNextSpawn))
        (if _is_spawn_valid
          (Utilities|Time|SetTimerbyFunctionName 0 "Spawn Enemy from Wave" _time)
          (Development|PrintString (Utilities|String|Append "Wave started, next spawn in " (Utilities|String|ToString(Float) _time) " seconds."))
          (else
            (Development|PrintString "No enemies for this wave")
            (CallFunction|EndWave)))))
    (else
      (Development|PrintString "Invalid Wave Number"))))

(fn AddResource
  (params (Resource%20Location :type Transform))
  (Utilities|Array|Add (Variables|Default|GetResource%20Locations) Resource%20Location)
  (Math|Integer|IncrementInt (Variables|Default|GetResource%20Amount%20%28Map%29)))

(fn RemoveResource
  (params (Resource%20Location :type Transform))
  (Utilities|Array|RemoveItem (Variables|Default|GetResource%20Locations) Resource%20Location)
  (Math|Integer|DecrementInt (Variables|Default|GetResource%20Amount%20%28Map%29)))

(fn AddResourcePlayer
  (params (Amount :type Integer))
  (Variables|Default|SetResource%20Amount%20%28Player%29 (+ Amount (Variables|Default|GetResource%20Amount%20%28Player%29)))
  (Development|PrintString (Utilities|String|ToString(Integer) (Variables|Default|GetResource%20Amount%20%28Player%29))))

(fn RemoveResourcePlayer
  (params (Amount :type Integer))
  (Variables|Default|SetResource%20Amount%20%28Player%29 (- (Variables|Default|GetResource%20Amount%20%28Player%29) Amount))
  (Development|PrintString (Utilities|String|ToString(Integer) (Variables|Default|GetResource%20Amount%20%28Player%29))))

(fn DefeatCheck)