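; Player controller for a mouse-driven tower defense game that adds the in-game menu to the viewport on BeginPlay.
; Left click spawns a Tower1 and Space spawns a BaseEnemy at the deprojected cursor position, flattened onto the Y=0 plane.
; Right click is a test toggle that shows and removes a PMSelection widget via FlipFlop.
; A noted bug has collision-adjusted tower spawns pushed outside neighboring towers' range radius.
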(event EventBeginPlay
  (Input|EnableInput 0)
  (bind _returnvalue (UserInterface|CreateWidget "/Game/Blueprints/UI/Ingame_Menu.Ingame_Menu_C"))
  (UserInterface|Viewport|AddtoViewport _returnvalue 0))

(event EventTick
  (params (DeltaSeconds :type Float%20%28single-precision%29)))

(event Input|MouseEvents|RightMouseButton
  (params (Key :type Key%20Structure :default "AnyKey"))
  ;[1 1 1] on click testing
  (:Pressed
    (Utilities|FlowControl|FlipFlop
      (:A
        (bind _returnvalue (UserInterface|CreateWidget "/Game/Blueprints/UI/PMSelection.PMSelection_C"))
        (UserInterface|Viewport|AddtoViewport _returnvalue 0)
        (Development|PrintString "widget's on"))
      (:B
        (Widget|RemovefromParent _returnvalue)
        (Development|PrintString "widget's gone again")))))

(event Input|MouseEvents|LeftMouseButton
  (params (Key :type Key%20Structure :default "AnyKey"))
  (bind _worldlocation (Game|Player|ConvertMouseLocationToWorldSpace))
  (bind (_x _y _z) (Math|Vector|BreakVector _worldlocation))
  (:Pressed
    ;[1 1 1] BUG: Something about colliding with the towers' range radius makes it so that if you try to spawn a tower near another one, it'll move to be outside of the towers' range if you have the collision handling set to be adjust to collisions
    (Game|SpawnActorfromClass "/Game/Blueprints/Towers/Tower1.Tower1_C" (Math|Transform|MakeTransform (Math|Vector|MakeVector _x 0.0 _z)) "Undefined" 0 0)))

(event Input|KeyboardEvents|SpaceBar
  (params (Key :type Key%20Structure :default "AnyKey"))
  (bind _worldlocation (Game|Player|ConvertMouseLocationToWorldSpace))
  (bind (_x _y _z) (Math|Vector|BreakVector _worldlocation))
  (:Pressed
    (Game|SpawnActorfromClass "/Game/Blueprints/Enemy/BaseEnemy.BaseEnemy_C" (Math|Transform|MakeTransform (Math|Vector|MakeVector _x 0.0 _z)) "Undefined" 0 0)))

(fn ConstructionScript)