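; TestKillzone is a test damage-zone actor that periodically hurts enemy-tagged actors overlapping it.
; BeginPlay starts a looping one-second timer that calls ApplyDamageOverTime by name.
; That function polls the overlapping actors and applies fixed damage to those tagged "enemy".
; Begin and end overlap events only print debug strings and play no part in the damage.
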(event EventBeginPlay
  (Utilities|Time|SetTimerbyFunctionName 0 "ApplyDamageOverTime" 1.0 true))

(event EventActorBeginOverlap
  (params (OtherActor :type Actor%20Object%20Reference))
  (Development|PrintString "Hello"))

(event EventTick
  (params (DeltaSeconds :type Float%20%28single-precision%29)))

(event Collision|EventActorEndOverlap
  (params (OtherActor :type Actor%20Object%20Reference))
  (Development|PrintString "Fuck"))

(fn ConstructionScript)

(fn ApplyDamageOverTime
  ;[1 1 1] Made with http://shootertutorial.com/2015/06/14/how-to-do-damage-advanced/
  (for _array_element (Collision|GetOverlappingActors 0 :!class /Script/Engine.Actor)
    (if (Actor|ActorHasTag _array_element "enemy")
      (Game|Damage|ApplyDamage _array_element 1e+01 0 0))))