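; Base tower for a tower defense game that turns toward and fires homing projectiles at enemies in range.
; Looping timers drive targeting, lerped rotation and shooting, with aim flattened to the tower's height.
; Targeting favors enemies nearest the GameState Objective, comparing against a stored minimum distance never reset here.
; Shooting drops targets that are invalid, out of range or would fall below zero health from one hit; hitscan firing is unused.
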(event EventBeginPlay
  (Utilities|Time|SetTimerbyFunctionName 0 "Find Closest Target" (Variables|Default|GetTarget%20Check%20Delay) true)
  (Utilities|Time|SetTimerbyFunctionName 0 "Rotate Towards Target" (Variables|Default|GetRotation%20Delay) true)
  (Utilities|Time|SetTimerbyFunctionName 0 "Shoot Enemy" (Variables|Default|GetFire%20Rate) true))

(event EventActorBeginOverlap
  (params (OtherActor :type Actor%20Object%20Reference)))

(event EventTick
  (params (DeltaSeconds :type Float%20%28single-precision%29)))

(fn ConstructionScript
  (|CallParentFunction))

(fn FireProjectile
  (params (Enemy%20Location :type Vector))
  (bind (_x _y) (Math|Vector|BreakVector Enemy%20Location))
  (bind _projectile_spawn_point (Variables|Default|GetProjectile%20Spawn%20Point))
  (bind _returnvalue (Transformation|GetWorldLocation _projectile_spawn_point))
  (bind _returnvalue_2 (Game|SpawnActorfromClass (Variables|Default|GetProjectileType) (Math|Transform|MakeTransform _returnvalue (Math|Rotator|FindLookatRotation _returnvalue (Math|Vector|MakeVector _x _y (.Z (Math|Vector|BreakVector _returnvalue))))) "AlwaysSpawn" 0 0))
  (if (Utilities|IsValid _returnvalue_2)
    (Default|SetHomingTarget _returnvalue_2 (Variables|Default|GetTargeted%20Enemy))))

(fn FindClosestTarget
  (bind _range (Variables|Default|GetRange))
  (bind _overlappingactors (Collision|GetOverlappingActors _range "/Game/Blueprints/Enemy/BaseEnemy.BaseEnemy_C" :!class /Script/Engine.PrimitiveComponent))
  (if (>= (Utilities|Array|LastIndex _overlappingactors) 0)
    (for _array_element _overlappingactors
      (bind _astdgame_state (Utilities|Casting|CastToTDGameState (Game|GetGameState)))
      (if (< (Transformation|GetDistanceTo (Variables|/Game/Blueprints/Gameplay/TDGameState.TDGameState_C|GetObjective _astdgame_state) _array_element) (LocalVariables|GetClosestEnemyDistance))
        (LocalVariables|SetClosestEnemyDistance (Transformation|GetDistanceTo (Variables|/Game/Blueprints/Gameplay/TDGameState.TDGameState_C|GetObjective _astdgame_state) _array_element))
        (Variables|Default|SetTargeted%20Enemy _array_element)))
    (Variables|Default|SetIsTargetingEnemy true)))

(fn CheckValidTarget
  (bind _range (Variables|Default|GetRange))
  (bind _targeted_enemy (Variables|Default|GetTargeted%20Enemy))
  (bind _overlappingactors (Collision|GetOverlappingActors _range "/Game/Blueprints/Enemy/BaseEnemy.BaseEnemy_C" :!class /Script/Engine.PrimitiveComponent))
  (bind _returnvalue (Utilities|IsValid _targeted_enemy))
  (bind _returnvalue_2 (Utilities|Array|ContainsItem _overlappingactors _targeted_enemy))
  (bind _returnvalue_3 (and _returnvalue_2 _returnvalue))
  (if _returnvalue_3
    ;[1 1 1] Check if the enemy would die after being shot
    (bind _asbase_enemy (Utilities|Casting|CastToBaseEnemy (Variables|Default|GetTargeted%20Enemy)))
    (return (>= (- (Variables|/Game/Blueprints/Enemy/BaseEnemy.BaseEnemy_C|GetHealth _asbase_enemy) (.ProjectileDamage (Utilities|GetClassDefaults (Variables|Default|GetProjectileType)))) 0.0))
    (else
      (return _returnvalue_3))))

(fn ShootEnemy
  ;[1 1 1] For targeting enemies https://www.youtube.com/watch?v=6iaT8LEi7iA https://answers.unrealengine.com/questions/103668/simple-blueprint-fireing-turret.html
  (Development|PrintString (Utilities|String|ToString(Boolean) (Variables|Default|GetIsTargetingEnemy)))
  (if (Variables|Default|GetIsTargetingEnemy)
    ;[1 1 1] Only shoot if there is still a valid target
    (bind _is_valid_target (CallFunction|CheckValidTarget))
    (if _is_valid_target
      ;;[1 1 1] Might want to make a hitscan bullet later
      (CallFunction|FireProjectile (Transformation|GetActorLocation (Variables|Default|GetTargeted%20Enemy)))
      (else
        (Variables|Default|SetIsTargetingEnemy false)
        (CallFunction|ShootEnemy)))))

(fn RotateTowardsTarget
  (bind _targeted_enemy (Variables|Default|GetTargeted%20Enemy))
  (bind _returnvalue (Transformation|GetActorLocation _targeted_enemy))
  (bind (_x _y) (Math|Vector|BreakVector _returnvalue))
  (if (and (Variables|Default|GetIsTargetingEnemy) (Utilities|IsValid (Variables|Default|GetTargeted%20Enemy)))
    (Transformation|SetActorRotation (Math|Rotator|Lerp(Rotator) (Transformation|GetActorRotation) (Math|Rotator|FindLookatRotation (Transformation|GetActorLocation) (Math|Vector|MakeVector _x _y (.Z (Math|Vector|BreakVector (Transformation|GetActorLocation))))) 0.3 true))))

(fn FireHitscan
  (params (Enemy%20Location :type Vector))
  (Collision|LineTraceByChannel (Transformation|GetWorldLocation (Variables|Default|GetProjectile%20Spawn%20Point)) Enemy%20Location "TraceTypeQuery1" false 0 "ForDuration")
  (Game|Damage|ApplyDamage (Variables|Default|GetTargeted%20Enemy) (Variables|Default|GetHitscan%20Damage) 0 0))