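; Tower1 is a turret Blueprint that automatically shoots BaseEnemy actors within its Range component.
; A looping FireRate timer calls Shoot Enemy, which fires at the locked target or picks another by horizontal distance when unlocked.
; Projectiles aim in the XZ plane, keeping the spawn point's Y for 2D shooting.
; The lock clears when the target is invalid, out of range, or predicted to die from the spawned projectile's damage.
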(event EventBeginPlay
  (Utilities|Time|SetTimerbyFunctionName 0 "Shoot Enemy" (Variables|Default|GetFire%20Rate) true))

(event EventActorBeginOverlap
  (params (OtherActor :type Actor%20Object%20Reference)))

(event EventTick
  (params (DeltaSeconds :type Float%20%28single-precision%29)))

(fn ConstructionScript
  (|CallParentFunction))

(fn FireProjectile
  (params (Enemy%20Location :type Vector))
  (bind (_x _y _z) (Math|Vector|BreakVector Enemy%20Location))
  (bind _projectile_spawn_point (Variables|Default|GetProjectile%20Spawn%20Point))
  (bind _returnvalue (Transformation|GetWorldLocation _projectile_spawn_point))
  (bind _returnvalue_2 (Game|SpawnActorfromClass (Variables|Default|GetProjectileType) (Math|Transform|MakeTransform _returnvalue (Math|Rotator|FindLookatRotation _returnvalue (Math|Vector|MakeVector _x (.Y (Math|Vector|BreakVector _returnvalue)) _z))) "AlwaysSpawn" 0 0))
  ;[1 1 1] If the enemy would die after being shot, set targeting check to be runnable again. This works reasonably well, but since I can only check if the enemy is still alive after the projectile is spawned, it will shoot more bullets until the enemy dies. Jank solution: Make the bullets fast enough to kill the enemy before the check happens again.
  (bind _asbase_enemy (Utilities|Casting|CastToBaseEnemy (Variables|Default|GetTargeted%20Enemy)))
  (if (<= (- (Variables|/Game/Blueprints/Enemy/BaseEnemy.BaseEnemy_C|GetHealth _asbase_enemy) (Variables|/Game/Blueprints/Towers/Projectiles/BaseProjectile.BaseProjectile_C|GetProjectileDamage _returnvalue_2)) 0.0)
    (Variables|Default|SetIsTargetingEnemy false)))

(fn FindClosestTarget
  (params (Targets :type Array%20of%20Actor%20Object%20References))
  (if (>= (Utilities|Array|LastIndex Targets) 0)
    (for _array_element Targets
      (if (< (Transformation|GetHorizontalDistanceTo _array_element) (LocalVariables|GetClosestEnemyDistance))
        (LocalVariables|SetClosestEnemyDistance (Transformation|GetHorizontalDistanceTo _array_element))
        (Variables|Default|SetTargeted%20Enemy _array_element)))
    (Variables|Default|SetIsTargetingEnemy true)
    (CallFunction|ShootEnemy)))

(event Custom|Shoot%20Enemy
  (bind _targeted_enemy (Variables|Default|GetTargeted%20Enemy))
  ;[1 1 1] For targeting enemies https://www.youtube.com/watch?v=6iaT8LEi7iA https://answers.unrealengine.com/questions/103668/simple-blueprint-fireing-turret.html
  (Development|PrintString (Utilities|String|ToString(Boolean) (Variables|Default|GetIsTargetingEnemy)))
  (if (Variables|Default|GetIsTargetingEnemy)
    ;[1 1 1] Only shoot if there is still a valid target
    (if (and (Utilities|Array|ContainsItem (Collision|GetOverlappingActors (Variables|Default|GetRange) "/Game/Blueprints/Enemy/BaseEnemy.BaseEnemy_C" :!class /Script/Engine.PrimitiveComponent) _targeted_enemy) (Utilities|IsValid _targeted_enemy))
      (CallFunction|FireProjectile (Transformation|GetActorLocation (Variables|Default|GetTargeted%20Enemy)))
      (else
        (Variables|Default|SetIsTargetingEnemy false)))
    (else
      (CallFunction|FindClosestTarget (Collision|GetOverlappingActors (Variables|Default|GetRange) "/Game/Blueprints/Enemy/BaseEnemy.BaseEnemy_C" :!class /Script/Engine.PrimitiveComponent)))))